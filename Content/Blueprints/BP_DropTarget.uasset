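; Drop target actor, apparently for a pinball-style game, labelled with its DropLetter through a text render set in the construction script.
; A hit calls Drop, which moves the mesh to a lowered relative position, disables its collision and plays the bumper hit sound.
; Reset re-enables collision, though its move uses the same lowered target location as Drop.
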(event `self.ReceiveBeginPlay`)

(event `Drop`
  (`KismetSystemLibrary.MoveComponentTo` (`self.DTMesh`) (0.0 0.0 -110.0))
  (`PrimitiveComponent.SetCollisionEnabled` (`self.DTMesh`) "NoCollision")
  (`GameplayStatics.PlaySoundAtLocation` "/Game/Assets/Sounds/BumperHit.BumperHit" (`self.K2_GetActorLocation`)))

(event `Reset`
  (`KismetSystemLibrary.MoveComponentTo` (`self.DTMesh`) (0.0 0.0 -110.0))
  (`PrimitiveComponent.SetCollisionEnabled` (`self.DTMesh`) "QueryAndPhysics"))

(event `EventHit`
  (`self.Drop`))

(fn `UserConstructionScript`
  (`TextRenderComponent.K2_SetText` (`self.TextRender`) (`KismetTextLibrary.Conv_StringToText` (`self.DropLetter`))))